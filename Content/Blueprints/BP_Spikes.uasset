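; BP_Spikes is a hazard actor that periodically damages the third-person player character while it stays within the spikes' box.
; On box overlap it caches the BP_ThirdPersonCharacter, if none is stored, and starts a looping half-second timer that calls ApplyPeriodicDamage.
; That event applies fixed damage to the cached character while it is valid.
; When the character leaves the box, the reference and timer are cleared.
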(event `self.Box.OnComponentBeginOverlap`
  (params (OverlappedComponent :type "PrimitiveComponent Object Reference") (OtherActor :type "Actor Object Reference") (OtherComp :type "PrimitiveComponent Object Reference") (OtherBodyIndex :type Integer) (bFromSweep :type Boolean) (SweepResult :type "HitResult Structure (by ref)"))
  (if (not (`KismetSystemLibrary.IsValid` (`self.BP_Player`)))
    (bind _asbp_third_person_character (cast `/Game/ThirdPerson/Blueprints/BP_ThirdPersonCharacter` OtherActor))
    (set `self.BP_Player` _asbp_third_person_character))
  (`KismetSystemLibrary.K2_SetTimer` null "ApplyPeriodicDamage" 0.5 true))

(event `self.Box.OnComponentEndOverlap`
  (params (OverlappedComponent :type "PrimitiveComponent Object Reference") (OtherActor :type "Actor Object Reference") (OtherComp :type "PrimitiveComponent Object Reference") (OtherBodyIndex :type Integer))
  (cast `/Game/ThirdPerson/Blueprints/BP_ThirdPersonCharacter` OtherActor)
  (set `self.BP_Player` null)
  (`KismetSystemLibrary.K2_ClearTimer` null "ApplyPeriodicDamage"))

(event `ApplyPeriodicDamage`
  (bind _bp_player (`self.BP_Player`))
  (if (`KismetSystemLibrary.IsValid` _bp_player)
    (`GameplayStatics.ApplyDamage` _bp_player 10.0)))

(fn `UserConstructionScript`)