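; Elevator actor that shuttles continuously between StartPoint and EndPoint, with no trigger.
; BeginPlay targets EndPoint, then Tick moves the actor toward the current target with VInterpTo, easing out as it approaches.
; Once within a small tolerance of the target, it switches to the opposite point without pausing.
; Movement does not sweep, so collisions do not block it.
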(event `self.ReceiveBeginPlay`
  (set `self.TargetPoint` (`self.EndPoint`)))

(event `self.ReceiveTick`
  (params (DeltaSeconds :type "Float (single-precision)"))
  (`self.K2_SetActorLocation` (`KismetMathLibrary.VInterpTo` (`self.K2_GetActorLocation`) (`self.TargetPoint`) (`GameplayStatics.GetWorldDeltaSeconds`) 2.0))
  (if (== (`self.K2_GetActorLocation`) (`self.TargetPoint`) :`ErrorTolerance` 1.0)
    (if (== (`self.TargetPoint`) (`self.StartPoint`) :`ErrorTolerance` 1.0)
      (set `self.TargetPoint` (`self.EndPoint`))
      (else
        (set `self.TargetPoint` (`self.StartPoint`))))))

(fn `UserConstructionScript`)