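; BP_Platform is a moving platform that travels to EndPoint while a BP_ThirdPersonCharacter is inside its Box trigger and returns to StartPoint otherwise.
; The Box overlap events store or clear the player reference and set IsMoving.
; Tick uses that flag to pick the target, easing the actor there with VInterpTo at MovementSpeed, without sweeping.
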(event `self.ReceiveBeginPlay`)

(event `self.ReceiveTick`
  (params (DeltaSeconds :type "Float (single-precision)"))
  (if (`self.IsMoving`)
    (`self.K2_SetActorLocation` (`KismetMathLibrary.VInterpTo` (`self.K2_GetActorLocation`) (`self.EndPoint`) (`GameplayStatics.GetWorldDeltaSeconds`) (`self.MovementSpeed`)))
    (else
      (`self.K2_SetActorLocation` (`KismetMathLibrary.VInterpTo` (`self.K2_GetActorLocation`) (`self.StartPoint`) (`GameplayStatics.GetWorldDeltaSeconds`) (`self.MovementSpeed`))))))

(event `self.Box.OnComponentBeginOverlap`
  (params (OverlappedComponent :type "PrimitiveComponent Object Reference") (OtherActor :type "Actor Object Reference") (OtherComp :type "PrimitiveComponent Object Reference") (OtherBodyIndex :type Integer) (bFromSweep :type Boolean) (SweepResult :type "HitResult Structure (by ref)"))
  (if (not (`KismetSystemLibrary.IsValid` (`self.BP_Player`)))
    (bind _asbp_third_person_character (cast `/Game/ThirdPerson/Blueprints/BP_ThirdPersonCharacter` OtherActor))
    (set `self.BP_Player` _asbp_third_person_character)
    (set `self.IsMoving` true)))

(event `self.Box.OnComponentEndOverlap`
  (params (OverlappedComponent :type "PrimitiveComponent Object Reference") (OtherActor :type "Actor Object Reference") (OtherComp :type "PrimitiveComponent Object Reference") (OtherBodyIndex :type Integer))
  (cast `/Game/ThirdPerson/Blueprints/BP_ThirdPersonCharacter` OtherActor)
  (set `self.BP_Player` null)
  (set `self.IsMoving` false))

(fn `UserConstructionScript`)